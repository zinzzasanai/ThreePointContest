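; TPC game mode that limits a play session with a countdown and returns to the FrontEnd level when time runs out.
; BeginPlay starts a looping one-second timer on CountdownGameTime, which decrements Countdown and prints it.
; At zero or below, a completion custom event calls ExitGame to open the level.
; The timer-clearing node is unconnected, so the timer is never explicitly stopped.
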(event Custom|Custom%20Event_CountdownCompleted
  (CallFunction|ExitGame))

(event EventBeginPlay
  (bind _returnvalue (Utilities|Time|SetTimerbyFunctionName 0 "CountdownGameTime" 1.0 true)))

(event EventTick
  (params (DeltaSeconds :type Float%20%28single-precision%29)))

(fn ConstructionScript)

(fn CountdownGameTime
  (Variables|Default|SetCountdown (- (Variables|Default|GetCountdown) 1))
  (Development|PrintString (Utilities|String|ToString(Integer) (Variables|Default|GetCountdown)))
  (if (<= (Variables|Default|GetCountdown) 0)
    (CallFunction|CustomEventCountdownCompleted)))

(fn ExitGame
  (Game|OpenLevel(byName) "FrontEnd"))